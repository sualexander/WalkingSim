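; BP_NPC is an interactable NPC that responds to the player with either a voice line or a dialogue.
; Its interaction event switches on an index, either playing the VoiceLineSwellGuy sound in 2D at slightly lowered pitch or starting DinerScene1Dialogue through BP_PlayerCharacter.
; BeginPlay, overlap, Tick and construction add no logic of their own.
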(event Custom|DoInteract_1
  (params (Index :type Integer))
  (switch int Index
    (:0
      (Audio|PlaySound2D "/Game/Sound/VoiceLineSwellGuy.VoiceLineSwellGuy" 1.0 0.925 0.0 0 0))
    (:1
      (bind _asbp_player_character (Utilities|Casting|CastToBP_PlayerCharacter (Game|GetPlayerCharacter 0)))
      (Default|StartDialogue _asbp_player_character "/Game/Dialogue/DinerScene1Dialogue.DinerScene1Dialogue"))))

(event EventBeginPlay
  (|CallParentFunction) ; This node is disabled and will not be called.\nDrag off pins to build functionality.
)

(event Collision|EventActorBeginOverlap
  (params (OtherActor :type Actor%20Object%20Reference)))

(event EventTick
  (params (DeltaSeconds :type Float%20%28single-precision%29))
  (|CallParentFunction DeltaSeconds) ; This node is disabled and will not be called.\nDrag off pins to build functionality.
)

(fn ConstructionScript
  (|CallParentFunction))