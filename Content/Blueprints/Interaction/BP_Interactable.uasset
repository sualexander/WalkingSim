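; Base interactable actor that shows a camera-tracking 3D text prompt and leaves DoInteract empty as a hook.
; The sphere collider shows the outer prompt and enables a Tick distance check against InnerRadius, which swaps to the inner prompt and enables player interaction.
; An encounter counter selects each prompt, and collision turns off once it exceeds the last outer prompt index.
; Optional debug spheres visualize both radii.
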(event OnComponentBeginOverlap(SphereCollider)
  (params (OverlappedComponent :type Primitive%20Component%20Object%20Reference) (OtherActor :type Actor%20Object%20Reference) (OtherComp :type Primitive%20Component%20Object%20Reference) (OtherBodyIndex :type Integer) (bFromSweep :type Boolean) (SweepResult :type Hit%20Result%20Structure%20%28by%20ref%29))
  (CallFunction|ShowOuter)
  (Variables|Default|SetbCheckInner true))

(event OnComponentEndOverlap(SphereCollider)
  (params (OverlappedComponent :type Primitive%20Component%20Object%20Reference) (OtherActor :type Actor%20Object%20Reference) (OtherComp :type Primitive%20Component%20Object%20Reference) (OtherBodyIndex :type Integer))
  (CallFunction|RemovePrompt)
  (Variables|Default|SetbCheckInner false))

(event Custom|ShowOuter
  (bind _outerwidget (Variables|Default|GetOuterWidget))
  (bind _prompt (Variables|/Game/Blueprints/UI/WBP_InteractPrompt.WBP_InteractPrompt_C|GetPrompt _outerwidget))
  (bind _prompt_2 (CallFunction|EvaluatePrompt (Variables|Default|GetPromptsOuter)))
  (Rendering|Components|TextRender|SetText _prompt _prompt_2)
  (UserInterface|SetWidget (Variables|Default|Get3DWidget) _outerwidget)
  (Rendering|SetVisibility (Variables|Default|Get3DWidget) true true)
  (Appearance|SetColorandOpacity _prompt (Utilities|Struct|MakeSlateColor "(R=1.000000,G=1.000000,B=1.000000,A=1.000000)" "UseColor_Specified") :!class /Script/UMG.TextBlock))

(event Custom|RemovePrompt
  (Rendering|SetVisibility (Variables|Default|Get3DWidget) false true))

(event Custom|DoInteract
  (params (Index :type Integer)))

(event Custom|ShowInner
  (bind _outerwidget (Variables|Default|GetOuterWidget))
  (bind _prompt (Variables|/Game/Blueprints/UI/WBP_InteractPrompt.WBP_InteractPrompt_C|GetPrompt _outerwidget))
  (bind _prompt_2 (CallFunction|EvaluatePrompt (Variables|Default|GetPromptsInner)))
  (Rendering|Components|TextRender|SetText _prompt _prompt_2)
  (UserInterface|SetWidget (Variables|Default|Get3DWidget) _outerwidget)
  (Appearance|SetColorandOpacity _prompt (Utilities|Struct|MakeSlateColor "(R=1.000000,G=1.000000,B=1.000000,A=1.000000)" "UseColor_Specified") :!class /Script/UMG.TextBlock))

(event Custom|StartInteract
  (params (Index :type Integer))
  (Development|PrintString "Interacted")
  (CallFunction|DoInteract Index)
  (CallFunction|RemovePrompt)
  (bind _result (Math|Integer|IncrementInt (Variables|Default|GetEncounters))
    (:%20%20
      (if (> _result (Utilities|Array|LastIndex (Variables|Default|GetPromptsOuter)))
        (Collision|SetActorEnableCollision false)
        (Development|PrintString "Exaughsted All Interactions")
        (Rendering|Debug|FlushPersistentDebugLines)))))

(event EventBeginPlay
  (bind _returnvalue (Transformation|GetActorLocation))
  (Utilities|FlowControl|Sequence
    (:then_0
      (bind _returnvalue_2 (UserInterface|CreateWidget "/Game/Blueprints/UI/WBP_InteractPrompt.WBP_InteractPrompt_C"))
      (Variables|Default|SetOuterWidget _returnvalue_2)
      (bind _returnvalue_3 (UserInterface|CreateWidget "/Game/Blueprints/UI/WBP_InteractPrompt.WBP_InteractPrompt_C"))
      (Variables|Default|SetInnerWidget _returnvalue_3)
      (Rendering|SetVisibility (Variables|Default|Get3DWidget) false false))
    (:then_1
      (Variables|Default|SetPlayerCamera (Game|GetPlayerCameraManager 0))
      (bind _asbp_player_character (Utilities|Casting|CastToBP_PlayerCharacter (Game|GetPlayerCharacter 0)))
      (Variables|Default|SetPlayer _asbp_player_character))
    (:then_2
      (if (Variables|Default|GetbDebug)
        (Rendering|Debug|DrawDebugSphere _returnvalue (Variables|Default|GetInnerRadius) 24 "(R=1.000000,G=0.000000,B=0.000000,A=1.000000)" 1e+03 0.5)
        (Rendering|Debug|DrawDebugSphere _returnvalue (Variables|/Script/Engine.SphereComponent|GetSphereRadius (Variables|Default|GetSphereCollider)) 24 "(R=1.000000,G=0.296445,B=0.000000,A=1.000000)" 1e+03 0.5)))))

(event EventTick
  (params (DeltaSeconds :type Float%20%28single-precision%29))
  (bind _returnvalue (Transformation|GetActorLocation))
  (bind _innerradius (Variables|Default|GetInnerRadius))
  (bind _playercamera (Variables|Default|GetPlayerCamera))
  (bind _player (Variables|Default|GetPlayer))
  (bind _returnvalue_2 (Camera|GetCameraLocation _playercamera))
  (bind _returnvalue_3 (Math|Vector|Distance(Vector) _returnvalue_2 _returnvalue))
  (bind _returnvalue_4 (< _returnvalue_3 _innerradius))
  (Utilities|FlowControl|Sequence
    (:then_0
      (Transformation|SetWorldRotation (Variables|Default|Get3DWidget) (Math|Rotator|MakeRotator 0.0 (* (.pitch (Camera|GetCameraRotation (Game|GetPlayerCameraManager 0))) -0.75) (.yaw (Math|Rotator|FindLookatRotation (Transformation|GetActorLocation) (Camera|GetCameraLocation (Variables|Default|GetPlayerCamera))))) false false))
    (:then_1
      (if (Variables|Default|GetbCheckInner)
        (if (Class|KismetMathLibrary|XORBoolean _returnvalue_4 (Variables|Default|GetbInInner))
          (bind _output_get (Variables|Default|SetbInInner _returnvalue_4))
          (if _output_get
            (CallFunction|ShowInner)
            (Default|EnableInteraction _player self)
            (else
              (CallFunction|ShowOuter)
              (Default|DisableInteraction _player))))))))

(fn ConstructionScript)

(fn EvaluatePrompt
  (params (Prompts :type Array%20of%20Texts))
  (return (Utilities|Array|Get(acopy) Prompts (Math|Integer|Clamp(Integer) (Variables|Default|GetEncounters) 0 (Utilities|Array|LastIndex Prompts)))))