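; Parent Blueprint for interactable items that the player can pick up into the inventory.
; On Pickup it passes the item to the player's inventory update, and on success hides the mesh, disables collision and tick, then clears both prompts after a brief delay.
; The actor is hidden rather than destroyed, and a failed update prints that the item is already in inventory.
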(event Custom|Pickup
  (params (Item :type S%20Item%20Structure))
  (bind _staticmesh (Variables|Default|GetStaticMesh))
  (bind _success (Default|UpdateInventory (Variables|Default|GetPlayer) Item))
  (if _success
    (Rendering|SetVisibility _staticmesh false false)
    (Collision|SetCollisionEnabled _staticmesh "NoCollision")
    (Actor|Tick|SetActorTickEnabled false)
    (Utilities|FlowControl|Delay 0.05)
    (CallFunction|ToggleInnerPrompt false)
    (CallFunction|ToggleOuterPrompt false)
    (else
      (Development|PrintText (Utilities|Text|FormatText "{item} already in inventory" (Utilities|Struct|BreakS_Item Item)) true true "(R=1.000000,G=0.382009,B=0.000000,A=1.000000)" 4.0))))

(fn ConstructionScript
  (|CallParentFunction))