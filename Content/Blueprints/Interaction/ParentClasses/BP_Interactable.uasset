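; Base interactable actor that shows outer and inner 3D prompts as the player approaches.
; A sphere collider gates Tick, which tracks Inner, Main and Outer distance bands, registers with the player, fades the outer prompt and turns widgets toward the camera.
; Prompts are filtered by encounter count and boolean conditions from local or player state.
; Clicking an inner prompt runs its indexed, mostly debug-print interaction, advances the count and refreshes the options.
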(event OnComponentBeginOverlap(SphereCollider)
  (params (OverlappedComponent :type Primitive%20Component%20Object%20Reference) (OtherActor :type Actor%20Object%20Reference) (OtherComp :type Primitive%20Component%20Object%20Reference) (OtherBodyIndex :type Integer) (bFromSweep :type Boolean) (SweepResult :type Hit%20Result%20Structure%20%28by%20ref%29))
  (Actor|Tick|SetActorTickEnabled true)
  (Development|PrintString (Utilities|String|Append "Enabled: " (Utilities|GetDisplayName self)) true true "(R=0.000000,G=1.000000,B=0.000000,A=1.000000)"))

(event OnComponentEndOverlap(SphereCollider)
  (params (OverlappedComponent :type Primitive%20Component%20Object%20Reference) (OtherActor :type Actor%20Object%20Reference) (OtherComp :type Primitive%20Component%20Object%20Reference) (OtherBodyIndex :type Integer))
  (Actor|Tick|SetActorTickEnabled false)
  (Development|PrintString (Utilities|String|Append "Disabled: " (Utilities|GetDisplayName self)) true true "(R=0.000000,G=0.000000,B=1.000000,A=1.000000)"))

(event Custom|ToggleOuterPrompt
  (params (bIsOn :type Boolean))
  (if bIsOn
    (bind _valid (CallFunction|EvaluatePrompts (Variables|Default|GetPromptsOuter)))
    (if (Utilities|Array|IsEmpty _valid)
      (Development|PrintText (Utilities|Text|FormatText "No more prompts available for {obj}" (Utilities|GetDisplayName self)) true true "(R=1.000000,G=0.000000,B=0.531469,A=1.000000)" 4.0)
      (Actor|Tick|SetActorTickEnabled false)
      (Collision|SetCollisionEnabled (Variables|Default|GetSphereCollider) "NoCollision")
      (else
        (Rendering|Components|TextRender|SetText (Variables|/Game/Blueprints/UI/WBP_OuterPrompt.WBP_OuterPrompt_C|GetPrompt (Variables|Default|GetOuterWidget)) (.text (Utilities|Array|Get(acopy) _valid)))
        (Rendering|SetVisibility (Variables|Default|Get3DWidgetOuter) true false)))
    (else
      (Rendering|SetVisibility (Variables|Default|Get3DWidgetOuter) false false))))

(event Custom|MainToOuter
  (Development|PrintString "MainToOuter"))

(event Custom|MainToInner
  (if (not (Variables|Default|GetbNoMoreInner))
    (Development|PrintString "MainToInner")
    (Default|AddInteractable (Variables|Default|GetPlayer) self)))

(event Custom|OuterTick
  (bind _mainradius (Variables|Default|GetMainRadius))
  ;[0 0 0] Tick
  (Widget|SetRenderOpacity (Variables|Default|GetOuterWidget) (Math|Float|MapRangeClamped (+ (/ (Math|Trig|Sin(Radians) (Math|Float|MultiplybyPi (- (- 1.0 (/ (- (Math|Vector|Distance(Vector) (Transformation|GetActorLocation (Variables|Default|GetPlayer)) (Transformation|GetActorLocation)) _mainradius) (- (Variables|Default|GetOuterRadius) _mainradius))) 0.5))) 2.0) 0.5) 0.0 1.0 0.1 1.0)))

(event Custom|CheckOverlap
  (bind _self self)
  (bind _returnvalue (Utilities|GetDisplayName _self))
  (if (Utilities|Array|IsEmpty (Collision|GetOverlappingActors "/Game/Blueprints/BP_PlayerCharacter.BP_PlayerCharacter_C" :!class /Script/Engine.Actor))
    (Actor|Tick|SetActorTickEnabled false)
    (Development|PrintString (Utilities|String|Append "Disabled: " _returnvalue) true true "(R=0.000000,G=0.000000,B=1.000000,A=1.000000)")
    (else
      (Actor|Tick|SetActorTickEnabled true)
      (Development|PrintString (Utilities|String|Append "Enabled: " _returnvalue) true true "(R=0.000000,G=1.000000,B=0.000000,A=1.000000)"))))

(event Custom|ToggleInnerPrompt
  (params (IsOn :type Boolean))
  (if IsOn
    (bind _valid (CallFunction|EvaluatePrompts (Variables|Default|GetPromptsInner)))
    (if (Utilities|Array|IsEmpty _valid)
      (CallFunction|InnertoMain)
      (Variables|Default|SetbNoMoreInner true)
      (Development|PrintText "No more inner prompts" true true "(R=1.000000,G=0.000000,B=0.531469,A=1.000000)" 4.0)
      (else
        (Default|UpdatePrompts (Variables|Default|GetInnerWidget) _valid)
        (Rendering|SetVisibility (Variables|Default|Get3DWidgetInner) true false)))
    (else
      (Rendering|SetVisibility (Variables|Default|Get3DWidgetInner) false false))))

(event Custom|InnerToMain
  (if (not (Variables|Default|GetbNoMoreInner))
    (Development|PrintString "InnerToMain")
    (Default|RemoveInteractable (Variables|Default|GetPlayer) self)))

(event Custom|OuterToMain
  (Development|PrintString "OuterToMain"))

(event Custom|InnerClicked
  (params (Prompt :type S%20Basic%20Prompt%20Structure))
  (CallFunction|Interactions (Utilities|Array|FindItem (Variables|Default|GetPromptsInner) Prompt))
  (CallFunction|ToggleInnerPrompt true)
  (Development|PrintString "Interacted"))

(event Custom|Interactions
  (params (Index :type Integer))
  (Math|Integer|IncrementInt (Variables|Default|GetEncounters)
    (:%20%20
      (switch int Index
        (:0
          (Development|PrintString "Inner 0-1"))
        (:1
          (Development|PrintString "Inner 0-2")
          (Utilities|Map|Add (Variables|/Game/Blueprints/BP_PlayerCharacter.BP_PlayerCharacter_C|GetAllBooleans (Variables|Default|GetPlayer)) "Inner 0-2" true))
        (:2
          (Development|PrintString "Inner 0-3"))
        (:3
          (Development|PrintString "Inner 1-1"))
        (:4
          (Development|PrintString "Inner 1-2"))
        (:5
          (Development|PrintString "Inner 2"))))))

(event EventBeginPlay
  (bind _outer (Variables|Default|GetOuter))
  (bind _main (Variables|Default|GetMain))
  (bind _3dwidgetouter (Variables|Default|Get3DWidgetOuter))
  (bind _sphereradius (Collision|GetComponentBounds _outer))
  (Utilities|FlowControl|Sequence
    (:then_0
      (Variables|Default|SetPlayerCamera (Game|GetPlayerCameraManager 0))
      (bind _asbp_player_character (Utilities|Casting|CastToBP_PlayerCharacter (Game|GetPlayerCharacter 0)))
      (Variables|Default|SetPlayer _asbp_player_character))
    (:then_1
      (bind _returnvalue (UserInterface|CreateWidget "/Game/Blueprints/UI/WBP_OuterPrompt.WBP_OuterPrompt_C"))
      (bind _output_get (Variables|Default|SetOuterWidget _returnvalue))
      (UserInterface|SetWidget _3dwidgetouter _output_get)
      (bind _returnvalue_2 (UserInterface|CreateWidget "/Game/Blueprints/UI/WBP_InteractPrompt.WBP_InteractPrompt_C"))
      (bind _output_get_2 (Variables|Default|SetInnerWidget _returnvalue_2))
      (UserInterface|SetWidget (Variables|Default|Get3DWidgetInner) _output_get_2)
      (EventDispatchers|BindEventtoOnClicked _output_get_2 (EventDispatchers|CreateEvent :!event Custom|InnerClicked))
      (Rendering|SetCastShadow _3dwidgetouter false))
    (:then_2
      (bind _isvalid (CallFunction|CheckPromptsLength))
      (if (not _isvalid)
        (Development|PrintText (Utilities|Text|FormatText "{obj}: InnerPrompts do not match OuterPrompts" (Utilities|GetDisplayName self)) true true "(R=1.000000,G=0.000000,B=0.000000,A=1.000000)" 4.0)))
    (:then_3
      (Variables|Default|SetInnerRadius (.SphereRadius (Collision|GetComponentBounds (Variables|Default|GetInner))))
      (Variables|Default|SetMainRadius (.SphereRadius (Collision|GetComponentBounds _main)))
      (Variables|Default|SetOuterRadius _sphereradius)
      (Components|Sphere|SetSphereRadius (Variables|Default|GetSphereCollider) (+ _sphereradius 1e+02) true)
      (CallFunction|CheckOverlap)
      (if (Variables|Default|GetbDoDebug)
        (Development|SetHiddeninGame _main false false)))))

(event EventTick
  (params (DeltaSeconds :type Float%20%28single-precision%29))
  (bind _returnvalue (Transformation|GetActorLocation))
  (bind _returnvalue_2 (Game|GetPlayerCameraManager 0))
  (bind _returnvalue_3 (Transformation|GetActorLocation))
  (bind _playercamera (Variables|Default|GetPlayerCamera))
  (bind _player (Variables|Default|GetPlayer))
  (bind _returnvalue_4 (Transformation|GetActorLocation _player))
  (bind _returnvalue_5 (Camera|GetCameraRotation _returnvalue_2))
  (bind _returnvalue_6 (Camera|GetCameraLocation _playercamera))
  (bind _returnvalue_7 (Math|Rotator|FindLookatRotation _returnvalue_3 _returnvalue_6))
  (bind _returnvalue_8 (Math|Vector|Distance(Vector) _returnvalue_4 _returnvalue))
  (bind _returnvalue_9 (* (.pitch _returnvalue_5) -0.75))
  ;[0 0 0] Tick
  (Utilities|FlowControl|Sequence
    (:then_0
      (if (< _returnvalue_8 (Variables|Default|GetInnerRadius))
        (if (Variables|Default|GetbInInner)
          ;;[1 1 1] Maybe
          (if (Variables|/Script/Engine.SceneComponent|GetbVisible (Variables|Default|Get3DWidgetOuter))
            (CallFunction|OuterTick))
          (else
            (Variables|Default|SetbInInner true)
            (Variables|Default|SetInMain false)
            (CallFunction|MaintoInner)))
        (elif (< _returnvalue_8 (Variables|Default|GetMainRadius))
          (if (not (Variables|Default|GetInMain))
            (Variables|Default|SetInMain true)
            (Variables|Default|SetbInOuter false)
            (if (Variables|Default|GetbInInner)
              (Variables|Default|SetbInInner false)
              (CallFunction|InnertoMain)
              (else
                (Variables|Default|SetbInInner false)
                (CallFunction|OutertoMain))))
          (elif (< _returnvalue_8 (Variables|Default|GetOuterRadius))
            (if (Variables|Default|GetbInOuter)
              (CallFunction|OuterTick)
              (else
                (Variables|Default|SetbInOuter true)
                (if (Variables|Default|GetInMain)
                  (Variables|Default|SetInMain false)
                  (CallFunction|MaintoOuter)
                  (else
                    (Variables|Default|SetInMain false)
                    (CallFunction|ToggleOuterPrompt true)))))
            (elif (Variables|Default|GetbInOuter)
              (Variables|Default|SetbInOuter false)
              (CallFunction|ToggleOuterPrompt false))))))
    (:then_1
      (if (or (Variables|Default|GetbInOuter) (Variables|Default|GetInMain))
        (Transformation|SetWorldRotation (Variables|Default|Get3DWidgetOuter) (Math|Rotator|MakeRotator 0.0 _returnvalue_9 (.yaw _returnvalue_7)) false false :!label _label)
        (elif (Variables|Default|GetbInInner)
          (Transformation|SetWorldRotation (Variables|Default|Get3DWidgetInner) (Math|Rotator|MakeRotator 0.0 _returnvalue_9 (.yaw _returnvalue_7)) false false)
          (if (Variables|/Script/Engine.SceneComponent|GetbVisible (Variables|Default|Get3DWidgetOuter))
            (goto _label)))))))

(fn ConstructionScript)

(fn EvaluatePrompts
  (params (Prompts :type Array%20of%20S%20Basic%20Prompt%20Structures))
  (for _array_element Prompts
    (if (== (.Encounters (Utilities|Struct|BreakS_BasicPrompt _array_element)) (Variables|Default|GetEncounters))
      (bind _output_get (LocalVariables|SetbConditionsValid true))
      (bind _keys (Utilities|Map|Keys (.Conditions (Utilities|Struct|BreakS_BasicPrompt _array_element))))
      (bind _array_element_2 (Utilities|Array|ForEachLoopwithBreak _keys :!label _label)
        (:LoopBody
          (if (.ReturnValue (Utilities|Map|Find (Variables|Default|GetLocalConditions) _array_element_2))
            (if (not (== (.Value (Utilities|Map|Find (.Conditions (Utilities|Struct|BreakS_BasicPrompt _array_element)) _array_element_2)) (.Value (Utilities|Map|Find (Variables|Default|GetLocalConditions) _array_element_2))))
              (LocalVariables|SetbConditionsValid false :!label _label_2)
              (goto _label Break))
            (elif (.ReturnValue (Utilities|Map|Find (Variables|/Game/Blueprints/BP_PlayerCharacter.BP_PlayerCharacter_C|GetAllBooleans (Variables|Default|GetPlayer)) _array_element_2))
              (if (not (== (.Value (Utilities|Map|Find (.Conditions (Utilities|Struct|BreakS_BasicPrompt _array_element)) _array_element_2)) (.Value (Utilities|Map|Find (Variables|/Game/Blueprints/BP_PlayerCharacter.BP_PlayerCharacter_C|GetAllBooleans (Variables|Default|GetPlayer)) _array_element_2))))
                (goto _label_2))
              (else
                (Development|PrintText (Utilities|Text|FormatText "Boolean {b} not found on player" _array_element_2) true true "(R=1.000000,G=0.379707,B=0.000000,A=1.000000)" 4.0)
                (goto _label_2)))))
        (:Completed
          (if _output_get
            (Utilities|Array|Add (LocalVariables|GetValidPrompts) _array_element))))))
  (return (LocalVariables|GetValidPrompts)))

(fn CheckPromptsLength
  (for _array_element (Variables|Default|GetPromptsOuter)
    (if (> (.Encounters (Utilities|Struct|BreakS_BasicPrompt _array_element)) (LocalVariables|GetMax))
      (LocalVariables|SetMax (.Encounters (Utilities|Struct|BreakS_BasicPrompt _array_element)))))
  (for _array_element_2 (Variables|Default|GetPromptsInner)
    (if (> (.Encounters (Utilities|Struct|BreakS_BasicPrompt _array_element_2)) (LocalVariables|GetMax))
      (return false)))
  (return true))