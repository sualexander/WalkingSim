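; BP_Stool is an interactable wooden stool that shows flavor text when the player examines it.
; The DoInteract_1 event switches on an Index to pick one of two descriptions.
; Each branch creates a WBP_TempText widget, sets its text, adds it to the viewport and removes it after a short delay.
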(event Custom|DoInteract_1
  (params (Index :type Integer))
  (switch int Index
    (:0
      (bind _returnvalue (UserInterface|CreateWidget "/Game/Blueprints/UI/WBP_TempText.WBP_TempText_C"))
      (Rendering|Components|TextRender|SetText (Variables|/Game/Blueprints/UI/WBP_TempText.WBP_TempText_C|GetTextBlock_33 _returnvalue) "Looks like a wooden stool")
      (UserInterface|Viewport|AddtoViewport _returnvalue 0)
      (Utilities|FlowControl|Delay 3.0)
      (Widget|RemovefromParent _returnvalue))
    (:1
      (bind _returnvalue_2 (UserInterface|CreateWidget "/Game/Blueprints/UI/WBP_TempText.WBP_TempText_C"))
      (Rendering|Components|TextRender|SetText (Variables|/Game/Blueprints/UI/WBP_TempText.WBP_TempText_C|GetTextBlock_33 _returnvalue_2) "Still just a stool")
      (UserInterface|Viewport|AddtoViewport _returnvalue_2 0)
      (Utilities|FlowControl|Delay 3.0)
      (Widget|RemovefromParent _returnvalue_2))))

(event EventBeginPlay
  (|CallParentFunction) ; This node is disabled and will not be called.\nDrag off pins to build functionality.
)

(event Collision|EventActorBeginOverlap
  (params (OtherActor :type Actor%20Object%20Reference)))

(event EventTick
  (params (DeltaSeconds :type Float%20%28single-precision%29))
  (|CallParentFunction DeltaSeconds) ; This node is disabled and will not be called.\nDrag off pins to build functionality.
)

(fn ConstructionScript
  (|CallParentFunction))