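; BP_Keys is an interactable keyring that responds to indexed interactions with subtitle text.
; On BeginPlay it creates a hidden WBP_TempText widget, which ShowText fills and displays for five seconds while incrementing an Encounters counter.
; The first interaction option only shows a description; the other two show their own lines, pick up a MechanicKey item and play a jingle sound.
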(event Custom|ShowText
  (params (InText :type Text))
  (bind _subtitle (Variables|Default|GetSubtitle))
  (Math|Integer|IncrementInt (Variables|Default|GetEncounters)
    (:%20%20
      (Rendering|Components|TextRender|SetText (Variables|/Game/Blueprints/UI/WBP_TempText.WBP_TempText_C|GetText _subtitle) InText)
      (Widget|SetVisibility _subtitle "Visible")
      (Utilities|FlowControl|Delay 5.0)
      (Widget|SetVisibility _subtitle "Collapsed"))))

(event EventInteractions
  (params (Index :type Integer))
  (bind _s_item (Utilities|Struct|MakeS_Item "MechanicKey"))
  (switch int Index
    (:0
      (CallFunction|ShowText "Just your run of the mill keyring. It's a wonder William can remember which key is used where."))
    (:1
      (CallFunction|ShowText "Found them keys")
      (CallFunction|Pickup _s_item)
      (Audio|PlaySound2D "/Game/Sound/KeysJingle.KeysJingle" 1.0 1.0 0.0 0 0 :!label _label))
    (:2
      (CallFunction|ShowText "I hope I don't get tetanus")
      (CallFunction|Pickup _s_item)
      (goto _label))))

(event EventBeginPlay
  (|CallParentFunction)
  (bind _returnvalue (UserInterface|CreateWidget "/Game/Blueprints/UI/WBP_TempText.WBP_TempText_C"))
  (bind _output_get (Variables|Default|SetSubtitle _returnvalue))
  (Widget|SetVisibility _output_get "Collapsed")
  (UserInterface|Viewport|AddtoViewport _output_get 0))

(fn ConstructionScript
  (|CallParentFunction))